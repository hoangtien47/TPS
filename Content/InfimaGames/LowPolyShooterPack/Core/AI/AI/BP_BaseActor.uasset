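; Base AI actor for the Low Poly Shooter Pack that takes damage and ragdolls on death.
; The Damage event subtracts from Health while it is above zero.
; When Health reaches zero or below, the Mesh switches to full physics simulation with physics-only collision.
; BeginPlay, Tick, overlap and the construction script do nothing, and a Health debug print is left disconnected.
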(event `self.Receive Damage`
  (params (Damage :type "Float (double-precision)"))
  (bind _mesh (`self.Mesh`))
  (if (> (`self.Health`) 0.0)
    (set `self.Health` (- (`self.Health`) Damage))
    (if (<= (`self.Health`) 0.0)
      (`PrimitiveComponent.SetSimulatePhysics` _mesh true)
      (`SkeletalMeshComponent.SetPhysicsBlendWeight` _mesh 1.0)
      (`PrimitiveComponent.SetCollisionEnabled` _mesh "PhysicsOnly"))))

(fn `UserConstructionScript`)