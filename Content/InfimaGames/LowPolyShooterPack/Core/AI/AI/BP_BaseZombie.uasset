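; BP_BaseZombie is the base zombie character, with damage, death and detection reactions plus hooks for movement speed and combat range.
; Any damage goes to ReceiveDamage; once Health is depleted, it detaches the controller and destroys the actor after a delay.
; Detect plays a scream montage on the mesh, and UpdateWalkSpeed sets the movement component's maximum walk speed.
; GetIdealRange returns zero strafe and attack radii.
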(event `self.ReceiveAnyDamage`
  (params (Damage :type "Float (single-precision)") (DamageType :type "DamageType Object Reference") (InstigatedBy :type "Controller Object Reference") (DamageCauser :type "Actor Object Reference"))
  (`self.Receive Damage` Damage)
  (if (<= (`self.Health`) 0.0)
    (`self.DetachFromControllerPendingDestroy`)
    (`KismetSystemLibrary.Delay` 10.0)
    (`self.K2_DestroyActor`)))

(event `/Game/AI/AI_Interface/BPI_Zombie.Detect`
  (`|PlayMontage` (`self.Mesh`) (`self.ScreamAnim`)))

(fn `GetIdealRange`
  (returns (StrafeRadius :type "Float (double-precision)") (AttackRadius :type "Float (double-precision)"))
  (return 0.0 0.0))

(fn `Update Walk Speed`
  (params (NewWalkSpeed :type "Float (double-precision)"))
  (set `CharacterMovementComponent.MaxWalkSpeed` NewWalkSpeed (`self.CharacterMovement`)))

(fn `UserConstructionScript`)