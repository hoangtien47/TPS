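; AI controller for zombie enemies that runs the possessed BP_BaseZombie's behavior tree and feeds it player detection state.
; On possess, it asks the pawn through a message call for its strafe and attack radii and writes them to the Blackboard.
; AI perception sets the player as enemy with line of sight and notifies the pawn once per detection.
; Otherwise, a timer delays clearing the target, line of sight and detected state.
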(event `self.ReceivePossess`
  (params (PossessedPawn :type "Pawn Object Reference"))
  (bind _asbp_base_zombie (cast `/Game/AI/BP_BaseZombie` PossessedPawn))
  (`self.RunBehaviorTree` (`/Game/AI/BP_BaseZombie.BT` _asbp_base_zombie))
  (bind (_straferadius _attackradius) (message `/Game/AI/AI_Interface/BPI_Zombie.GetIdealRange` PossessedPawn))
  (`BlackboardComponent.SetValueAsFloat` (`self.Blackboard`) (`self.StrafeRadius`) _straferadius)
  (`BlackboardComponent.SetValueAsFloat` (`self.Blackboard`) (`self.AttackRadius`) _attackradius))

(event `self.AIPerception.OnTargetPerceptionUpdated`
  (params (Actor :type "Actor Object Reference") (Stimulus :type "AIStimulus Structure"))
  (bind _blackboard (`self.Blackboard`))
  (if (and (`self.ActorHasTag` Actor "Player") (`.bSuccessfullySensed` (break `AIStimulus` Stimulus)))
    (set `self.Enemy` Actor)
    (`KismetSystemLibrary.K2_ClearAndInvalidateTimerHandle` (`self.EnemyTimer`))
    (`BlackboardComponent.SetValueAsBool` _blackboard (`self.HasLineOfSight`) true)
    (`BlackboardComponent.SetValueAsObject` _blackboard (`self.EnemyActor`) Actor)
    (if (not (`self.IsDetected`))
      (message `/Game/AI/AI_Interface/BPI_Zombie.Detect` (`self.K2_GetPawn`))
      (set `self.IsDetected` true))
    (else
      (bind _returnvalue (`KismetSystemLibrary.K2_SetTimerDelegate` (delegate `StartEnemyTimer`) (`self.Line Of Sight Timer`)))
      (set `self.EnemyTimer` _returnvalue))))

(event `StartEnemyTimer`
  (bind _blackboard (`self.Blackboard`))
  (`BlackboardComponent.SetValueAsBool` _blackboard (`self.HasLineOfSight`) false)
  (`BlackboardComponent.SetValueAsObject` _blackboard (`self.EnemyActor`) null)
  (set `self.IsDetected` false))

(fn `UserConstructionScript`)