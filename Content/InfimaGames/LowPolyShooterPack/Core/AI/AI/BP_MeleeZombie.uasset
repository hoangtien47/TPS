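; Melee zombie AI character that attacks by playing a montage and damaging a pawn in front of it.
; On the montage's notify begin, a short forward sphere trace against pawns applies damage to the hit actor, with debug drawing left on.
; GetIdealRange supplies fixed strafe and attack radii, with attack range much closer than strafe range.
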(event `/Game/AI/AI_Interface/BPI_Zombie.Attack`
  (bind _returnvalue (`self.K2_GetActorLocation`))
  (bind _notifyname (`|PlayMontage` (`self.Mesh`) (`self.AttackMontage`))
    (:`OnNotifyBegin`
      (switch `name` _notifyname
        (:`Attack`
          (bind (_outhit _returnvalue_2) (`KismetSystemLibrary.SphereTraceSingleForObjects` :`Start` _returnvalue :`End` (+ _returnvalue (* (`self.GetActorForwardVector`) 150.0)) :`Radius` 20.0 :`ObjectTypes` (`|MakeArray` "ObjectTypeQuery3" :!type "EObjectTypeQuery Enum") :`DrawDebugType` "ForDuration"))
          (if _returnvalue_2
            (`GameplayStatics.ApplyDamage` (`.HitActor` (`GameplayStatics.BreakHitResult` _outhit)) (`self.Damage`))))))))

(fn `GetIdealRange`
  (returns (StrafeRadius :type "Float (double-precision)") (AttackRadius :type "Float (double-precision)"))
  (return 300.0 50.0))

(fn `UserConstructionScript`)