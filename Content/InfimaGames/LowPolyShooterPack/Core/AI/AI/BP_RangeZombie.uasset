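; BP_RangeZombie is a ranged zombie enemy that attacks with a gun and reports its ideal strafe and attack radii through GetIdealRange.
; Attack plays gun and body animations, and the montage notify fires a debug-drawn forward line trace that damages the hit actor.
; AnyDamage passes damage to ReceiveDamage; at zero health it detaches the controller and destroys the actor after a delay.
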(event `self.Attack`
  (bind _returnvalue (`self.K2_GetActorLocation`))
  (`SkeletalMeshComponent.PlayAnimation` (`self.Gun`) (`self.FireAnim`) false)
  (bind _notifyname (`|PlayMontage` (`self.Mesh`) (`self.AttackMontage`))
    (:`OnNotifyBegin`
      (switch `name` _notifyname
        (:`Attack`
          (bind (_outhit _returnvalue_2) (`KismetSystemLibrary.LineTraceSingle` :`Start` _returnvalue :`End` (+ _returnvalue (* (`self.GetActorForwardVector`) 800.0)) :`TraceChannel` "TraceTypeQuery3" :`DrawDebugType` "ForDuration"))
          (if _returnvalue_2
            (`GameplayStatics.ApplyDamage` (`.HitActor` (`GameplayStatics.BreakHitResult` _outhit)) (`self.Damage`))))))))

(event `self.ReceiveAnyDamage`
  (params (Damage :type "Float (single-precision)") (DamageType :type "DamageType Object Reference") (InstigatedBy :type "Controller Object Reference") (DamageCauser :type "Actor Object Reference"))
  (`self.Receive Damage` Damage)
  (if (<= (`self.Health`) 0.0)
    (`self.DetachFromControllerPendingDestroy`)
    (`KismetSystemLibrary.Delay` 5.0)
    (`self.K2_DestroyActor`)))

(fn `GetIdealRange`
  (returns (StrafeRadius :type "Float (double-precision)") (AttackRadius :type "Float (double-precision)"))
  (return 600.0 600.0))

(fn `UserConstructionScript`)